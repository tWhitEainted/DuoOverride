(event EventInteract
  (if (or (Variables|Default|GetCanPressE) (Variables|Default|GetEnemyCanOpen))
    (if (Variables|Default|GetCanInteract)
      (Variables|Default|SetCanInteract false)
      (if (Variables|Default|GetEngaged)
        (Variables|Default|SetEngaged false)
        (else
          (Variables|Default|SetEngaged false)
          (Development|PrintString "Box interacted")
          (Utilities|FlowControl|Delay 0.2)
          (bind _asbp_player_character (Utilities|Casting|CastToBP_PlayerCharacter (Variables|Default|GetPlayerInstance)))
          (Default|StartQTE _asbp_player_character)
          (Variables|Default|SetCanInteract true))))))

(fn ConstructionScript
  (|CallParentFunction))